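; BP_BasicEnemy is a basic enemy that loses health when hit by projectiles and is destroyed when that health runs out.
; BeginPlay sets Health in its GeneralCharacterInfo struct to MaxHealth.
; On a capsule hit by a BP_Projectile, IsDead tests whether the projectile's Damage would be lethal, then the enemy either destroys itself or subtracts it via DamageEnemy.
; The projectile is destroyed after either outcome.
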(event `self.ReceiveBeginPlay`
  (set `/Game/Blueprints/GeneralCharacterInfo.Health` (`self.MaxHealth`) (`self.GeneralCharacterInfo`)))

(event `self.CapsuleComponent.OnComponentHit`
  (params (HitComponent :type "PrimitiveComponent Object Reference") (OtherActor :type "Actor Object Reference") (OtherComp :type "PrimitiveComponent Object Reference") (NormalImpulse :type "Vector Structure") (Hit :type "HitResult Structure (by ref)"))
  (if (== (`GameplayStatics.GetObjectClass` OtherActor) "/Game/Blueprints/Projectiles/BP_Projectile.BP_Projectile_C")
    (bind _asbp_projectile (cast `/Game/Blueprints/Projectiles/BP_Projectile` OtherActor))
    (bind _damage (`/Game/Blueprints/Projectiles/BP_Projectile.Damage` _asbp_projectile))
    (bind _isdead (`self.IsDead` _damage))
    (if _isdead
      (`self.K2_DestroyActor`)
      (else
        (`self.DamageEnemy` _damage)))
    (`self.K2_DestroyActor` OtherActor)))

(fn `DamageEnemy`
  (params (Damage :type Integer))
  (bind _generalcharacterinfo (`self.GeneralCharacterInfo`))
  (set `/Game/Blueprints/GeneralCharacterInfo.Health` (- (`/Game/Blueprints/GeneralCharacterInfo.Health` _generalcharacterinfo) Damage) _generalcharacterinfo))

(fn `IsDead`
  (params (Damage :type Integer))
  (returns (IsDead :type Boolean))
  (return (<= (- (`/Game/Blueprints/GeneralCharacterInfo.Health` (`self.GeneralCharacterInfo`)) Damage) 0)))

(fn `UserConstructionScript`)