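; GeneralCharacterInfo is a Blueprint that stores a character's Health and MaxHealth and exposes functions to change them, with no active event logic.
; GetHit subtracts damage only if Health stays above zero, so lethal hits change nothing.
; Heal clamps only when the heal amount alone exceeds MaxHealth, so Health can overshoot it.
; AddHealth and RemoveHealth shift both values together, with removal setting either to 1 instead of zero or below.
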(fn `AddHealth`
  (params (`Health Amount To Add` :type Integer))
  (set `self.Health` (+ `Health Amount To Add` (`self.Health`)))
  (set `self.MaxHealth` (+ (`self.MaxHealth`) (`local.Health Amount To Add`))))

(fn `GetHit`
  (params (Damage :type Integer))
  (bind _health (`self.Health`))
  (if (> (- _health Damage) 0)
    (set `self.Health` (- _health Damage))))

(fn `Heal`
  (params (HealAmount :type Integer))
  (if (== (`self.Health`) (`self.MaxHealth`))
    _
    (elif (> (`local.HealAmount`) (`self.MaxHealth`))
      (set `self.Health` (`self.MaxHealth`))
      (else
        (set `self.Health` (+ (`self.Health`) (`local.HealAmount`)))))))

(fn `RemoveHealth`
  (params (HealthToRemove :type Integer))
  (bind _returnvalue (- (`self.MaxHealth`) HealthToRemove))
  (bind _returnvalue_2 (- (`self.Health`) HealthToRemove))
  (`|ExecutionSequence`
    (:`then_0`
      (if (<= _returnvalue_2 0)
        (set `self.Health` 1)
        (else
          (set `self.Health` _returnvalue_2))))
    (:`then_1`
      (if (<= _returnvalue 0)
        (set `self.MaxHealth` 1)
        (else
          (set `self.MaxHealth` _returnvalue))))))