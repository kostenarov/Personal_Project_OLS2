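; BP_TestItem is a test inventory item actor that can be looked at to show a pickup prompt.
; LookAt uses the ItemID in its ItemDataComponent to find a data table row and returns "Pick up" text with the item's name.
; When destroyed, it adds itself to the ActorsRemoved list in the third-person game mode's level save data.
; BeginPlay only runs a one-second delay with nothing after it.
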(event `self.ReceiveBeginPlay`
  (`KismetSystemLibrary.Delay` 1.0))

(event `self.ReceiveDestroyed`
  (bind _asbp_third_person_game_mode (cast `/Game/Blueprints/BP_ThirdPersonGameMode` (`GameplayStatics.GetGameMode`)))
  (`KismetArrayLibrary.Array_AddUnique` (`/Game/Blueprints/SaveData_LevelData.ActorsRemoved` (`/Game/Blueprints/BP_ThirdPersonGameMode.As Save Data Level Data` _asbp_third_person_game_mode)) (`|ConvertAsset` self)))

(fn `LookAt`
  (returns (Message :type Text))
  (bind (_itemid_datatable _itemid_rowname) (break `DataTableRowHandle` (`/Game/Blueprints/Inventory/ItemDataComponent.itemID` (`self.ItemDataComponent`))))
  (bind _returnvalue (`|GetDataTableRow` _itemid_datatable _itemid_rowname)
    (:`then`
      (return (`|FormatText` "Pick up {Item}" (`.Name_2_9A7FAB5C40292D9AEAAE4EA14DB53893` (break `/Game/Blueprints/Inventory/F_ItemStruct` _returnvalue)))))))

(fn `UserConstructionScript`)