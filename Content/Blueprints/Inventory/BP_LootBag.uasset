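; BP_LootBag is a loot bag actor that holds items in an InventorySystem component and removes itself once emptied.
; On each inventory update it checks the quantity; at zero or below it takes the HUD Menu of player controller 0 off its parent, then destroys the actor.
; The destroy only runs if that controller casts to BP_PlayerController, and the construction script just calls its parent.
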(event `self.InventorySystem.OnInventoryUpdated`
  (if (<= (`/Game/Blueprints/Inventory/InventorySystem.GetQuantity` (`self.InventorySystem`)) 0)
    (bind _asbp_player_controller (cast `/Game/Blueprints/BP_PlayerController` (`GameplayStatics.GetPlayerController` 0)))
    (`Widget.RemoveFromParent` (`/Game/Blueprints/W_PlayerHUD.Menu` (`/Game/Blueprints/BP_PlayerController.HUD` _asbp_player_controller)))
    (`self.K2_DestroyActor`)))

(fn `UserConstructionScript`
  (`parent.UserConstructionScript`))