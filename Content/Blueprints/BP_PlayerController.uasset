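; Player controller that creates the player's hot bar and HUD widgets and handles inventory input.
; On BeginPlay, only for the local controller, it creates both widgets, stores them in variables and adds them to the viewport.
; The IA_Inventory Enhanced Input action, on Started, calls DisplayPlayerMenu on the HUD widget to show the player menu.
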(event `self.ReceiveBeginPlay`
  (if (`self.IsLocalPlayerController`)
    (bind _returnvalue (`|CreateWidget` "/Game/Blueprints/Inventory/UI/W_HotBar.W_HotBar_C"))
    (bind _output_get (set `self.HotBar` _returnvalue))
    (`UserWidget.AddToViewport` _output_get 0)
    (bind _returnvalue_2 (`|CreateWidget` "/Game/Blueprints/W_PlayerHUD.W_PlayerHUD_C"))
    (bind _output_get_2 (set `self.HUD` _returnvalue_2))
    (`UserWidget.AddToViewport` _output_get_2 0)))

(event `EnhancedInput|/Game/Blueprints/Input/Actions/IA_Inventory`
  (params (ActionValue :type Boolean) (ElapsedSeconds :type "Float (double-precision)") (TriggeredSeconds :type "Float (double-precision)") (InputAction :type "InputAction Object Reference" :default "/Game/Blueprints/Input/Actions/IA_Inventory.IA_Inventory"))
  (:`Started`
    (`/Game/Blueprints/W_PlayerHUD.DisplayPlayerMenu` (`self.HUD`))))

(fn `UserConstructionScript`)