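; Pickup actor that represents an equipment item in the world and prompts the player when in range.
; On BeginPlay a child actor component takes the class of its Item.
; Sphere overlap by the third-person character shows a notification widget with a generated thumbnail of that class and enables CanPickUp.
; Leaving the sphere removes the widget and clears the flag; the pickup itself is not handled in this graph.
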(event `self.ReceiveBeginPlay`
  (`ChildActorComponent.SetChildActorClass` (`self.BP_Item`) (`GameplayStatics.GetObjectClass` (`self.Item`))))

(event `self.Sphere.OnComponentBeginOverlap`
  (params (OverlappedComponent :type "PrimitiveComponent Object Reference") (OtherActor :type "Actor Object Reference") (OtherComp :type "PrimitiveComponent Object Reference") (OtherBodyIndex :type Integer) (bFromSweep :type Boolean) (SweepResult :type "HitResult Structure (by ref)"))
  (bind _asbp_third_person_character (cast `/Game/Blueprints/BP_ThirdPersonCharacter` OtherActor))
  (bind _returnvalue (`|CreateWidget` "/Game/Blueprints/UI/BP_PickUpNotif.BP_PickUpNotif_C"))
  (bind _output_get (set `self.UI_Ref` _returnvalue))
  (bind _thumbnail (`|GenerateThumbnail` (`GameplayStatics.GetObjectClass` (`self.Item`)) (struct) null)
    (:`then`
      (`Image.SetBrushFromTexture` (`/Game/Blueprints/UI/BP_PickUpNotif.Thumbnail` _output_get) _thumbnail false)
      (`UserWidget.AddToViewport` _output_get 0)
      (set `/Game/Blueprints/BP_ThirdPersonCharacter.Can Pick Up` true _asbp_third_person_character))))

(event `self.Sphere.OnComponentEndOverlap`
  (params (OverlappedComponent :type "PrimitiveComponent Object Reference") (OtherActor :type "Actor Object Reference") (OtherComp :type "PrimitiveComponent Object Reference") (OtherBodyIndex :type Integer))
  (bind _asbp_third_person_character (cast `/Game/Blueprints/BP_ThirdPersonCharacter` OtherActor))
  (`Widget.RemoveFromParent` (`self.UI_Ref`))
  (set `/Game/Blueprints/BP_ThirdPersonCharacter.Can Pick Up` false _asbp_third_person_character))

(fn `Destroy Actor`
  (`self.K2_DestroyActor`))

(fn `GetItem`
  (returns (BP_Item :type "/Game/Blueprints/Equipment/BP_Item Object Reference"))
  (return null))

(fn `UserConstructionScript`)