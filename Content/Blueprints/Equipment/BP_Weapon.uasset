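; Weapon equipment Blueprint that casts a configurable projectile, with its Type enum set in the construction script after the parent's runs.
; SetProjectile stores the class that Cast spawns at the world transform of the passed Direction component, adjusting for collision but always spawning.
; Cast sets the projectile root's scale to Size and divides its max speed by Size, copying that to initial speed, so bigger shots get lower speed values.
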(fn `Cast`
  (params (Direction :type "ArrowComponent Object Reference") (Size :type "Float (double-precision)"))
  (bind _returnvalue (`|SpawnActorFromClass` (`self.Projectile`) (`SceneComponent.K2_GetComponentToWorld` Direction) "AdjustIfPossibleButAlwaysSpawn" "MultiplyWithRoot" null null))
  (`SceneComponent.SetWorldScale3D` (`/Game/Blueprints/Projectiles/BP_Projectile.DefaultSceneRoot` _returnvalue) (`KismetMathLibrary.Conv_DoubleToVector` Size))
  (bind _projectilemovement (`/Game/Blueprints/Projectiles/BP_Projectile.ProjectileMovement` _returnvalue))
  (bind _output_get (set `ProjectileMovementComponent.MaxSpeed` (/ (`MovementComponent.GetMaxSpeed` _projectilemovement) Size) _projectilemovement))
  (set `ProjectileMovementComponent.InitialSpeed` _output_get _projectilemovement))

(fn `SetProjectile`
  (params (Projectile :type "/Game/Blueprints/Projectiles/BP_Projectile Class Reference"))
  (set `self.Projectile` Projectile))

(fn `UserConstructionScript`
  (`parent.UserConstructionScript`)
  (set `self.Type` "NewEnumerator1"))