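; BP_Weapon_Fire is a weapon Blueprint whose Cast function launches a projectile, spawning BP_Projectile_Ice despite the Fire name.
; Cast spawns it at the given component's transform, scales its mesh by ProjectileSize, and divides max speed by that size.
; InitialSpeed is set to the new max speed after spawning, so larger projectiles are meant to travel slower.
; The event graph only prints a debug string on actor overlap.
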(event `self.ReceiveActorBeginOverlap`
  (params (OtherActor :type "Actor Object Reference"))
  (`KismetSystemLibrary.PrintString` "colided"))

(fn `Cast`
  (params (`Spawn location` :type "ArrowComponent Object Reference") (`Projectile Size` :type "Float (double-precision)"))
  (bind _returnvalue (`|SpawnActorFromClass` "/Game/Blueprints/BP_Projectile_Ice.BP_Projectile_Ice_C" (`SceneComponent.K2_GetComponentToWorld` `Spawn location`) "AdjustIfPossibleButAlwaysSpawn" "MultiplyWithRoot" null null))
  (`SceneComponent.SetWorldScale3D` (`/Game/Blueprints/BP_Projectile_Ice.StaticMesh` _returnvalue) (`KismetMathLibrary.Conv_DoubleToVector` `Projectile Size`))
  (bind _projectilemovement (`/Game/Blueprints/BP_Projectile_Ice.ProjectileMovement` _returnvalue))
  (bind _output_get (set `ProjectileMovementComponent.MaxSpeed` (/ (`MovementComponent.GetMaxSpeed` _projectilemovement) `Projectile Size`) _projectilemovement))
  (set `ProjectileMovementComponent.InitialSpeed` _output_get _projectilemovement))

(fn `UserConstructionScript`)